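; Player controller for the simple ship that forwards player input to the BP_SimpleShip pawn.
; BeginPlay caches player 0's pawn as the ship, and the MoveThrust axis sets its throttle.
; Both tilt axis events share one assignment to the ship's controller rotation, deriving opposite-signed pitch and roll from a single axis value, with zero yaw.
; Tick only stores delta time.
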(event `self.ReceiveBeginPlay`
  ;[1 1 1] Begin
  (bind _asbp_simple_ship (cast `/Game/Blueprints/BP_SimpleShip` (`GameplayStatics.GetPlayerPawn` 0)))
  (set `self.Ship` _asbp_simple_ship))

(event `InputAction|GrabObject`
  ;[1 1 1] GRAB
)

(event `self.ReceiveTick`
  (params (DeltaSeconds :type "Float (single-precision)"))
  ;[1 1 1] TICK
  (set `self.delta_time` DeltaSeconds))

(event `InputAxis|MoveThrust`
  (params (AxisValue :type "Float (single-precision)"))
  ;[1 1 1] Thrust
  (set `/Game/Blueprints/BP_SimpleShip.ThrottleAxis` AxisValue (`self.Ship`)))

(event `InputAxis|MoveTiltAway`
  (params (AxisValue :type "Float (single-precision)"))
  ;[1 1 1] Rotatio
  (set `/Game/Blueprints/BP_SimpleShip.ControllerRotation` (`KismetMathLibrary.MakeRot` (* AxisValue -50.0) 0.0 (* (stale `InputAxis|MoveTiltRight` AxisValue) 50.0)) (`self.Ship`) :!label _label))

(event `InputAxis|MoveTiltRight`
  (params (AxisValue :type "Float (single-precision)"))
  ;[1 1 1] Rotatio
  (goto _label))

(fn `UserConstructionScript`)