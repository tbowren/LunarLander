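; BP_2048Tile is a tile actor for a 2048 game that shows a number and slides to its target position.
; Tick uses VInterpTo to ease the actor toward TargetLocation, with a DoOnce tied to recording CurrentLocation and printing a debug position.
; UpdateUI writes Value into the Widget_TileText widget, and DeleteMe destroys the tile after a one-second delay.
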(event `self.ReceiveBeginPlay`)

(event `UpdateUI`
  (bind _aswidget_tile_text (cast `/Game/Blueprints/Widget_TileText` (`WidgetComponent.GetUserWidgetObject` (`self.Widget`))))
  (`TextBlock.SetText` (`/Game/Blueprints/Widget_TileText.TXT_Value` _aswidget_tile_text) (`KismetTextLibrary.Conv_IntToText` (`self.Value`))))

(event `self.ReceiveActorBeginOverlap`
  (params (OtherActor :type "Actor Object Reference")))

(event `self.ReceiveTick`
  (params (DeltaSeconds :type "Float (single-precision)"))
  (bind _returnvalue (`self.K2_GetActorLocation`))
  (bind _targetlocation (`self.TargetLocation`))
  (if (!= _returnvalue _targetlocation)
    (`self.K2_SetActorLocation` (`KismetMathLibrary.VInterpTo` _returnvalue (`self.TargetLocation`) DeltaSeconds 12.0))
    (`/Engine/EditorBlueprintResources/StandardMacros.DoOnce` false :!via `Reset`
      (:`Completed`
        (set `self.CurrentLocation` _targetlocation)
        (`KismetSystemLibrary.PrintString` (`KismetStringLibrary.Concat_StrStr` "tiLE: " (`KismetStringLibrary.Conv_VectorToString` _returnvalue)))))))

(event `DeleteMe`
  (`KismetSystemLibrary.Delay` 1.0)
  (`self.K2_DestroyActor`))

(fn `UserConstructionScript`)