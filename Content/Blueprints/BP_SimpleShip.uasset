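; Lander-style ship with a physics thruster that burns fuel, carries cargo and can crash.
; Tick eases rotation toward the controller target, scales thrust, flame and audio by throttle, and updates fuel and cargo HUD bars.
; A downward trace gives altitude for stepped camera zoom and speed-based crash detection, which notifies TransferGameMode and enables click-to-restart.
; Functions adjust fuel and cargo for transfers; safe-landing scoring is disconnected.
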(event `Key|Gamepad_FaceButton_Bottom`
  (bind _ball (`self.Ball`))
  ;[1 1 1] Restart after crash
  (:`Pressed`
    (if (`self.isClickedToRestart`) :!label _label
      (set `self.isCrashed` false)
      (set `self.isLanded` false)
      (set `self.isClickedToRestart` false)
      (`SceneComponent.K2_SetWorldLocation` _ball (`self.StartLocation`) false)
      (`PrimitiveComponent.SetMaterial` _ball 0 "/Game/Materials/M_Ship.M_Ship"))))

(event `Key|LeftMouseButton`
  ;[1 1 1] Restart after crash
  (:`Pressed`
    (goto _label)))

(event `self.ReceiveTick`
  (params (DeltaSeconds :type "Float (single-precision)"))
  (bind _ball (`self.Ball`))
  (bind _springarm (`self.SpringArm`))
  (bind _throttleaxis (`self.ThrottleAxis`))
  (bind _returnvalue (`SceneComponent.GetComponentVelocity` (`self.Ball`)))
  (bind _returnvalue_2 (`SceneComponent.K2_GetComponentLocation` (`self.Ball`)))
  (bind _returnvalue_3 (- (`self.Fuel`) (* (* DeltaSeconds (`self.ThrottleAxis`)) (`self.Inefficiency`))))
  (if (`self.isCrashed`)
    ;[1 1 1] Crashed
    (`PrimitiveComponent.SetMaterial` (`self.Ball`) 0 "/Game/Materials/M_Ship_Red.M_Ship_Red")
    (set `PhysicsThrusterComponent.ThrustStrength` 0.0 (`self.PhysicsThruster`))
    (`SceneComponent.SetRelativeScale3D` (`self.ThrustPivot`) (1.0 1.0 0.0))
    (else
      (`SceneComponent.K2_SetWorldRotation` _ball (`KismetMathLibrary.RInterpTo` (`SceneComponent.K2_GetComponentRotation` _ball) (`self.ControllerRotation`) DeltaSeconds (`self.ShipRotate Drag`)) false)
      ;[1 1 1] Time
      (set `self.Time` (+ (`self.Time`) DeltaSeconds))
      ;[1 1 1] Make sure we have fuel in tank but dont go negative
      (if (< _returnvalue_3 0.0)
        (set `self.Fuel` 0.0)
        (else
          (set `self.Fuel` _returnvalue_3)
          ;[1 1 1] Scale and show engine Thrust
          (set `PhysicsThrusterComponent.ThrustStrength` (* (`self.ThrustForce`) _throttleaxis -1.0) (`self.PhysicsThruster`))
          (`SceneComponent.SetRelativeScale3D` (`self.ThrustPivot`) (`KismetMathLibrary.MakeVector` 1.0 1.0 (* _throttleaxis 3.0)))
          ;[1 1 1] Audio
          (`AudioComponent.SetVolumeMultiplier` (`self.Engine_Thrust`) _throttleaxis)))
      ;[1 1 1] Update HUD
      (bind _aswidget_fuel (cast `/Game/Blueprints/Widget_Fuel` (`WidgetComponent.GetUserWidgetObject` (`self.Widget`))))
      (if (not (`self.isCrashed`))
        (`ProgressBar.SetPercent` (`/Game/Blueprints/Widget_Fuel.PB_Fuel` _aswidget_fuel) (/ (`self.Fuel`) (`self.MaxFuel`)))
        (`ProgressBar.SetPercent` (`/Game/Blueprints/Widget_Fuel.PB_Cargo` _aswidget_fuel) (/ (`self.Cargo`) (`self.MaxCargo`)))
        ;[1 1 1] Get Altitude
        (bind _outhit (`KismetSystemLibrary.LineTraceSingle` _returnvalue_2 (- _returnvalue_2 (0.0 0.0 30000.0)) "TraceTypeQuery1"))
        (bind (_bblockinghit _binitialoverlap _time _location _impactpoint _normal _impactnormal _physmat _hitactor _hitcomponent _hitbonename _hititem _tracestart) (`GameplayStatics.BreakHitResult` _outhit))
        (bind _output_get (set `self.Altitude` (`KismetMathLibrary.VSize` (- _tracestart _impactpoint))))
        (if (> _output_get 12000.0)
          (set `SpringArmComponent.TargetArmLength` 24000.0 _springarm)
          (elif (< _output_get 5000.0)
            (set `SpringArmComponent.TargetArmLength` 5000.0 _springarm)
            (if (< _output_get 128.0)
              ;[1 1 1] Crassh or Safe Land
              (if (> (`KismetMathLibrary.VSize` _returnvalue) 750.0)
                (`KismetSystemLibrary.PrintString` "CRASH")
                (set `self.Fuel` 0.0)
                (set `self.isCrashed` true)
                (set `self.CrashedVel` _returnvalue)
                (set `self.ThrottleAxis` 0.0)
                (`/Game/Blueprints/TransferGameMode.Crashed` (`self.GameMode`))
                (`KismetSystemLibrary.Delay` 2.0)
                (set `self.isClickedToRestart` true)))
            (else
              (set `SpringArmComponent.TargetArmLength` 12000.0 _springarm))))))))

(event `self.ReceiveBeginPlay`
  ;[1 1 1] BEGIN
  (bind _astransfer_game_mode (cast `/Game/Blueprints/TransferGameMode` (`GameplayStatics.GetGameMode`)))
  (set `self.GameMode` _astransfer_game_mode)
  (set `self.StartLocation` (`self.K2_GetActorLocation`)))

(fn `SendCargo`
  (params (NewParam :type "Float (double-precision)"))
  (returns (CargoOut :type "Float (double-precision)"))
  ;[1 1 1] Make sure not over filled
  (bind _output_get (set `self.Cargo` (+ NewParam (`self.Cargo`))))
  (if (>= _output_get (`self.MaxCargo`))
    (bind _output_get_2 (set `self.FuelTken` NewParam))
    (else
      (set `self.FuelTken` 0.0)))
  (return _output_get_2))

(fn `SendPower`
  (params (NewParam :type "Float (double-precision)"))
  (returns (PowerOut :type "Float (double-precision)"))
  (bind _maxfuel (`self.MaxFuel`))
  ;[1 1 1] Make sure not over filled
  (bind _output_get (set `self.Fuel` (+ NewParam (`self.Fuel`))))
  (if (>= _output_get _maxfuel)
    (set `self.Fuel` _maxfuel)
    (else
      (bind _output_get_2 (set `self.FuelTken` NewParam))))
  (return _output_get_2))

(fn `TransferCargo`
  (params (NewParam :type "Float (double-precision)"))
  (returns (NewParam1 :type "Float (double-precision)"))
  (bind _cargo (`self.Cargo`))
  (bind _returnvalue (`KismetMathLibrary.Abs` (`self.Amount_to_Transfer`)))
  (bind _output_get (set `self.Amount_to_Transfer` NewParam))
  ;[1 1 1] if value is positive, moving cargo to ship
  (if (not (> _output_get 0.0))
    ;[1 1 1] if negative,  taking cargo OFF ship
    (if (< (`self.Amount_to_Transfer`) 0.0)
      ;[1 1 1] Do we have enough cargo to send?
      (if (< _returnvalue _cargo)
        (set `self.Cargo` (- _cargo _returnvalue))
        (else
          ;[1 1 1] if no, send whatever we have
          (bind _output_get_2 (set `self.Amount_to_Transfer` (* _cargo -1.0)))
          (set `self.Cargo` 0.0)))))
  (return _output_get_2))

(fn `UserConstructionScript`)