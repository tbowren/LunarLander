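; BP_PowerEmitter is a power station that sends stored power and cargo to an overlapping actor through interface messages.
; Overlap events toggle sending, and Tick transfers both at a shared frame-time-scaled rate while updating the widget's fuel bar.
; Power recharges up to its maximum when idle or after a successful transfer, but stalls if too low to send.
; The green-button binding is disconnected, and the emitter's own send/transfer functions are empty stubs.
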(event `self.ReceiveBeginPlay`
  (bind _aswidget_fuel (cast `/Game/Blueprints/Widget_Fuel` (`WidgetComponent.GetUserWidgetObject` (`self.Widget`))))
  (`Widget.SetVisibility` (`/Game/Blueprints/Widget_Fuel.PB_Cargo` _aswidget_fuel) "Hidden"))

(event `greenclick`
  (`KismetSystemLibrary.PrintString` "Hello")
  (set `self.PowerStorage` (`self.MaxFuelStorage`)))

(event `self.ReceiveActorBeginOverlap`
  (params (OtherActor :type "Actor Object Reference"))
  ;[1 1 1] overlap events
  (set `self.isSendingPower` true))

(event `self.ReceiveActorEndOverlap`
  (params (OtherActor :type "Actor Object Reference"))
  ;[1 1 1] overlap events
  (set `self.isSendingPower` false))

(event `self.ReceiveTick`
  (params (DeltaSeconds :type "Float (single-precision)"))
  (bind _powerstorage (`self.PowerStorage`))
  (bind _cargostorage (`self.CargoStorage`))
  (bind _returnvalue (* (`self.TransferEnergyRate`) DeltaSeconds))
  (bind _returnvalue_2 (* (`self.TransferEnergyRate`) DeltaSeconds))
  (bind _returnvalue_3 (- (`self.PowerStorage`) _returnvalue))
  (bind _aswidget_fuel (cast `/Game/Blueprints/Widget_Fuel` (`WidgetComponent.GetUserWidgetObject` (`self.Widget`))))
  ;[1 1 1] updates Fuel Widget
  (`ProgressBar.SetPercent` (`/Game/Blueprints/Widget_Fuel.PB_Fuel` _aswidget_fuel) (/ (`self.PowerStorage`) (`self.MaxFuelStorage`)))
  ;[1 1 1] If transfering power make sure we have some, then transfer
  (if (`self.isSendingPower`)
    (`|ExecutionSequence`
      (:`then_0`
        (if (> _returnvalue_3 0.0)
          (message `/Game/Blueprints/BPI_Emission.SendPower` (stale `self.ReceiveActorBeginOverlap` OtherActor) _returnvalue)
          (set `self.PowerStorage` _returnvalue_3)
          ;[1 1 1] power strorage is not yet full so add to it
          (if (< _powerstorage (`self.MaxFuelStorage`)) :!label _label
            (set `self.PowerStorage` (+ _powerstorage (* DeltaSeconds (`self.ChargeRate`)))))))
      (:`then_1`
        ;[1 1 1] Cargo
        (if (> _cargostorage 0.0)
          (message `/Game/Blueprints/BPI_Emission.SendCargo` (stale `self.ReceiveActorBeginOverlap` OtherActor) _returnvalue_2)
          (set `self.CargoStorage` (- _cargostorage _returnvalue_2)))))
    (else
      (goto _label))))

(fn `SendCargo`
  (params (NewParam :type "Float (double-precision)"))
  (returns (CargoOut :type "Float (double-precision)"))
  (return 0.0))

(fn `SendPower`
  (params (NewParam :type "Float (double-precision)"))
  (returns (PowerOut :type "Float (double-precision)"))
  (return 0.0))

(fn `TransferCargo`
  (params (NewParam :type "Float (double-precision)"))
  (returns (NewParam1 :type "Float (double-precision)"))
  (return 0.0))

(fn `UserConstructionScript`)