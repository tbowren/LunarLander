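; BP_curve is an actor that animates a grid of static mesh cubes in a wave driven by a float curve.
; BeginPlay creates the mesh components.
; Tick sets world positions from grid indices, summing row and column curve samples over a height that rises per row.
; Curve time advances a fixed step per frame, independent of delta time, and resets past half the curve's maximum time.
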(event `self.ReceiveBeginPlay`
  (for _ (range (+ (`self.CubeCount`) 1))
    (bind _returnvalue (`AddComponent|Static Mesh Component_895`))
    (`KismetArrayLibrary.Array_Add` (`self.CubeArray`) _returnvalue)))

(event `self.ReceiveTick`
  (params (DeltaSeconds :type "Float (single-precision)"))
  (bind _arraygridlength (`self.ArrayGridLength`))
  (bind _curvetime (`self.CurveTime`))
  (bind _returnvalue (+ (`self.CurveTime`) (`self.Curve_Step`)))
  (for (_array_element _array_index) (`self.CubeArray`)
    (bind _returnvalue_2 (/ _array_index _arraygridlength))
    (bind _returnvalue_3 (`KismetMathLibrary.Conv_IntToDouble` _returnvalue_2))
    (bind _returnvalue_4 (mod _array_index _arraygridlength))
    (`SceneComponent.K2_SetWorldLocation` _array_element (`KismetMathLibrary.MakeVector` (* _returnvalue_3 500.0) (* (`KismetMathLibrary.Conv_IntToDouble` _returnvalue_4) 500.0 1.0) (+ (* (`CurveFloat.GetFloatValue` (`self.curve`) (+ (* (`KismetMathLibrary.Conv_IntToDouble` _returnvalue_4) (`self.CubeNeighborStep`) 1.0) _curvetime)) (`self.FloatTravelHeight`)) 100.0 (* _returnvalue_3 200.0) (* (`CurveFloat.GetFloatValue` (`self.curve`) (+ (* (`KismetMathLibrary.Conv_IntToDouble` _returnvalue_2) 0.05 1.0) _curvetime)) 250.0))) false))
  ;[1 1 1] Comment
  (if (<= _returnvalue (/ (`.MaxTime` (`CurveBase.GetTimeRange` (`self.curve`))) 2.0))
    (set `self.CurveTime` _returnvalue)
    (else
      (set `self.CurveTime` 0.0))))

(fn `UserConstructionScript`)