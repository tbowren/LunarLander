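; BP_Physics is a Blueprint that moves a Cube component with hand-written force, mass and velocity math.
; BeginPlay sets velocity from StartForce over Mass, then Tick moves the cube unswept and adds Gravity over Mass, scaled by delta time.
; Below a hard-coded floor height, it clamps Z and adds the start impulse to the current velocity.
; Left and Right key presses add sideways impulses along Y, also divided by Mass.
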(event `Key|Right`
  (:`Pressed`
    (set `self.DeltaVelocity` (+ (`self.DeltaVelocity`) (/ (0.0 40.0 0.0) (`self.Mass`))))))

(event `Key|Left` :consume false
  (:`Pressed`
    (set `self.DeltaVelocity` (+ (`self.DeltaVelocity`) (/ (0.0 -40.0 0.0) (`self.Mass`))))))

(event `self.ReceiveActorBeginOverlap`
  (params (OtherActor :type "Actor Object Reference")))

(event `self.ReceiveBeginPlay`
  (set `self.DeltaVelocity` (/ (`self.StartForce`) (`self.Mass`))))

(event `self.ReceiveTick`
  (params (DeltaSeconds :type "Float (single-precision)"))
  (bind _cube (`self.Cube`))
  (bind _returnvalue (`SceneComponent.K2_GetComponentLocation` _cube))
  (`SceneComponent.K2_AddWorldTransform` (`self.Cube`) (`KismetMathLibrary.Conv_VectorToTransform` (* (`self.DeltaVelocity`) DeltaSeconds)) false)
  (set `self.DeltaVelocity` (+ (`self.DeltaVelocity`) (/ (* (`self.Gravity`) DeltaSeconds) (`self.Mass`))))
  ;[1 1 1] if below ground reset force
  (if (< (.z _returnvalue) 170.0)
    (`SceneComponent.K2_SetWorldLocation` _cube (`KismetMathLibrary.MakeVector` (.x _returnvalue) (.y _returnvalue) 170.0) false)
    (set `self.DeltaVelocity` (+ (`self.DeltaVelocity`) (/ (`self.StartForce`) (`self.Mass`))))))

(fn `UserConstructionScript`)