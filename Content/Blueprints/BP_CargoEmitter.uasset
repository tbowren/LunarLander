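; Cargo emitter actor that stores self-replenishing cargo and transfers it to an overlapping actor.
; Overlap events toggle sending, and Tick passes a rate-scaled amount through SendCargoMessage, deducts it and recharges storage up to its maximum.
; Recharge also runs when idle, but not while sending with too little cargo.
; A Widget_Fuel bar shows the fill level; power and upgrade-button logic is left unwired.
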(event `self.ReceiveBeginPlay`
  (bind _aswidget_fuel (cast `/Game/Blueprints/Widget_Fuel` (`WidgetComponent.GetUserWidgetObject` (`self.Widget`))))
  (`Widget.SetVisibility` (`/Game/Blueprints/Widget_Fuel.PB_Fuel` _aswidget_fuel) "Hidden")
  (`ProgressBar.SetFillColorAndOpacity` (`/Game/Blueprints/Widget_Fuel.PB_Cargo` _aswidget_fuel) (`KismetMathLibrary.MakeColor` 0.0 0.0 1.0)))

(event `greenclick`
  (`KismetSystemLibrary.PrintString` "Hello")
  (set `self.PowerStorage` (`self.MaxFuelStorage`)))

(event `self.ReceiveActorBeginOverlap`
  (params (OtherActor :type "Actor Object Reference"))
  ;[1 1 1] overlap events
  (set `self.isSendingPower` true))

(event `self.ReceiveActorEndOverlap`
  (params (OtherActor :type "Actor Object Reference"))
  ;[1 1 1] overlap events
  (set `self.isSendingPower` false))

(event `self.ReceiveTick`
  (params (DeltaSeconds :type "Float (single-precision)"))
  (bind _cargostorage (`self.CargoStorage`))
  (bind _returnvalue (* (`self.TransferEnergyRate`) DeltaSeconds))
  (bind _returnvalue_2 (- (`self.CargoStorage`) _returnvalue))
  ;[1 1 1] updates Fuel Widget
  (bind _aswidget_fuel (cast `/Game/Blueprints/Widget_Fuel` (`WidgetComponent.GetUserWidgetObject` (`self.Widget`))))
  (`ProgressBar.SetPercent` (`/Game/Blueprints/Widget_Fuel.PB_Cargo` _aswidget_fuel) (/ (`self.CargoStorage`) (`self.MaxCargoStorage`)))
  ;[1 1 1] If transfering power make sure we have some, then transfer
  (if (`self.isSendingPower`)
    (`|ExecutionSequence`
      (:`then_0`
        (if (> _returnvalue_2 0.0)
          (message `/Game/Blueprints/BPI_Emission.SendCargo` (stale `self.ReceiveActorBeginOverlap` OtherActor) _returnvalue)
          (set `self.CargoStorage` _returnvalue_2)
          ;[1 1 1] power strorage is not yet full so add to it
          (if (< _cargostorage (`self.MaxCargoStorage`)) :!label _label
            (set `self.CargoStorage` (+ _cargostorage (* DeltaSeconds (`self.ChargeRate`))))))))
    (else
      (goto _label))))

(fn `SendCargo`
  (params (NewParam :type "Float (double-precision)"))
  (returns (CargoOut :type "Float (double-precision)"))
  (return 0.0))

(fn `SendPower`
  (params (NewParam :type "Float (double-precision)"))
  (returns (PowerOut :type "Float (double-precision)"))
  (return 0.0))

(fn `TransferCargo`
  (params (NewParam :type "Float (double-precision)"))
  (returns (NewParam1 :type "Float (double-precision)"))
  (return 0.0))

(fn `UserConstructionScript`)