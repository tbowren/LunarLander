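; Player ship for an arcade game: a thruster-driven craft that manages fuel and cargo and can carry physics objects.
; Thrust input drives engine force, flame scale, audio and fuel burn; Tick also recharges fuel and updates widgets.
; Key taps step pitch and roll, applied each Tick, and Space levels the ship.
; Grab traces downward and holds the hit component below with a physics handle; separate functions handle cargo and power transfers.
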(event `self.ReceiveTick`
  (params (DeltaSeconds :type "Float (single-precision)"))
  (bind _maxfuel (`self.MaxFuel`))
  (bind _returnvalue (/ (`self.Fuel`) (`self.MaxFuel`)))
  (`SceneComponent.K2_SetWorldRotation` (`self.Ball`) (`KismetMathLibrary.MakeRot` (`self.RotAway`) 0.0 (`self.RotRight`)) false)
  (bind _returnvalue_2 (- (`self.Fuel`) (* (* DeltaSeconds (stale `InputAxis|MoveThrust` AxisValue)) (`self.Inefficiency`))))
  ;[1 1 1] Make sure we have fuel in tank but dont go negative
  (if (< _returnvalue_2 0.0)
    (set `self.Fuel` 0.0))
  (bind _returnvalue_3 (+ (`self.ChargeRate`) _returnvalue_2))
  ;[1 1 1] Make sure we dont over fill tank
  (if (< _returnvalue_3 _maxfuel)
    (set `self.Fuel` _returnvalue_3)
    (else
      (set `self.Fuel` _maxfuel)))
  ;[1 1 1] Update HUD
  (bind _aswidget_fuel (cast `/Game/Blueprints/Widget_Fuel` (`WidgetComponent.GetUserWidgetObject` (`self.Widget`))))
  (bind _aswidget_hud (cast `/Game/Blueprints/Widget_HUD` (`WidgetComponent.GetUserWidgetObject` (`self.Widget_HUD`))))
  (`ProgressBar.SetPercent` (`/Game/Blueprints/Widget_Fuel.PB_Fuel` _aswidget_fuel) _returnvalue)
  (`ProgressBar.SetPercent` (`/Game/Blueprints/Widget_Fuel.PB_Cargo` _aswidget_fuel) (/ (`self.Cargo`) (`self.MaxCargo`)))
  (`TextBlock.SetText` (`/Game/Blueprints/Widget_HUD.TXT_FuelPercent` _aswidget_hud) (`KismetTextLibrary.Conv_DoubleToText` (`KismetMathLibrary.Conv_IntToDouble` (`KismetMathLibrary.Round` (* 100 _returnvalue))) "HalfToEven"))
  (if (`self.isGrabbed`)
    (`PhysicsHandleComponent.SetTargetLocationAndRotation` :`self` (`self.PhysicsHandle`) :`NewLocation` (+ (`SceneComponent.K2_GetComponentLocation` (`self.Ball`)) (0.0 0.0 -500.0)))))

(event `self.ReceiveBeginPlay`
  ;[1 1 1] Comment
  (set `self.MaxFuel` (`self.Fuel`)))

(event `InputAction|GrabObject`
  (bind _returnvalue (`SceneComponent.K2_GetComponentLocation` (`self.Ball`)))
  ;[1 1 1] Grab
  (:`Pressed`
    (set `self.isGrabbed` true)
    (bind _outhit (`KismetSystemLibrary.LineTraceSingleForObjects` :`Start` _returnvalue :`End` (+ _returnvalue (0.0 0.0 -1000.0)) :`ObjectTypes` (`self.PhysicsObjectTypes`) :`DrawDebugType` "ForDuration"))
    (bind _returnvalue_2 (`AddComponent|Physics Handle Component_1`))
    (set `self.PhysicsHandle` _returnvalue_2)
    (bind (_bblockinghit _binitialoverlap _time _location _impactpoint _normal _impactnormal _physmat _hitactor _hitcomponent) (`GameplayStatics.BreakHitResult` _outhit))
    (set `self.PhysicsObject` _hitcomponent)
    (`PhysicsHandleComponent.GrabComponent` (`self.PhysicsHandle`) _hitcomponent "None" _location true))
  (:`Released`
    (set `self.isGrabbed` false)
    (`PhysicsHandleComponent.ReleaseComponent` (`self.PhysicsHandle`))))

(event `InputAxis|MoveThrust`
  (params (AxisValue :type "Float (single-precision)"))
  (bind _returnvalue (`KismetMathLibrary.FClamp` AxisValue))
  ;[1 1 1] Thrust
  ;[1 1 1] Scale and show engine Thrust
  (set `PhysicsThrusterComponent.ThrustStrength` (* (`self.ThrustForce`) _returnvalue -1.0) (`self.PhysicsThruster`))
  (`SceneComponent.SetRelativeScale3D` (`self.ThrustPivot`) (`KismetMathLibrary.MakeVector` 1.0 1.0 (* _returnvalue 3.0)))
  ;[1 1 1] Audio
  (`AudioComponent.SetVolumeMultiplier` (`self.Engine_Thrust`) AxisValue))

(event `Key|S`
  ;[1 1 1] Roll / Tilt
  (:`Pressed`
    (set `self.RotAway` (+ (`self.RotAway`) 5.0))))

(event `InputAxis|MoveTiltAway`
  (params (AxisValue :type "Float (single-precision)"))
  ;[1 1 1] Roll / Tilt
  (if (> AxisValue 0.5)
    _))

(event `Key|W`
  ;[1 1 1] Roll / Tilt
  (:`Pressed`
    (set `self.RotAway` (+ (`self.RotAway`) -5.0))))

(event `Key|Right`
  ;[1 1 1] Roll / Tilt
  (:`Pressed`
    (set `self.RotRight` (+ (`self.RotRight`) 5.0) :!label _label)))

(event `Key|D`
  ;[1 1 1] Roll / Tilt
  (:`Pressed`
    (goto _label)))

(event `InputAxis|MoveTiltRight`
  (params (AxisValue :type "Float (single-precision)"))
  ;[1 1 1] Roll / Tilt
  (if (> AxisValue 0.7)
    _
    (elif (< AxisValue -0.7)
      _)))

(event `Key|A`
  (:`Pressed`
    (set `self.RotRight` (+ (`self.RotRight`) -5.0) :!label _label_2)))

(event `Key|Left`
  (:`Pressed`
    (goto _label_2)))

(event `Key|Down`)

(event `Key|SpaceBar`
  (:`Pressed`
    (bind _output_get (set `self.RotAway` 0.0))
    (bind _output_get_2 (set `self.RotRight` 0.0))
    (set `self.isAbort` true)))

(fn `SendCargo`
  (params (NewParam :type "Float (double-precision)"))
  (returns (CargoOut :type "Float (double-precision)"))
  ;[1 1 1] Make sure not over filled
  (bind _output_get (set `self.Cargo` (+ NewParam (`self.Cargo`))))
  (if (>= _output_get (`self.MaxCargo`))
    (bind _output_get_2 (set `self.FuelTken` NewParam))
    (else
      (set `self.FuelTken` 0.0)))
  (return _output_get_2))

(fn `SendPower`
  (params (NewParam :type "Float (double-precision)"))
  (returns (PowerOut :type "Float (double-precision)"))
  (bind _maxfuel (`self.MaxFuel`))
  ;[1 1 1] Make sure not over filled
  (bind _output_get (set `self.Fuel` (+ NewParam (`self.Fuel`))))
  (if (>= _output_get _maxfuel)
    (set `self.Fuel` _maxfuel)
    (else
      (bind _output_get_2 (set `self.FuelTken` NewParam))))
  (return _output_get_2))

(fn `TransferCargo`
  (params (NewParam :type "Float (double-precision)"))
  (returns (NewParam1 :type "Float (double-precision)"))
  (bind _cargo (`self.Cargo`))
  (bind _returnvalue (`KismetMathLibrary.Abs` (`self.Amount_to_Transfer`)))
  (bind _output_get (set `self.Amount_to_Transfer` NewParam))
  ;[1 1 1] if value is positive, moving cargo to ship
  (if (not (> _output_get 0.0))
    ;[1 1 1] if negative,  taking cargo OFF ship
    (if (< (`self.Amount_to_Transfer`) 0.0)
      ;[1 1 1] Do we have enough cargo to send?
      (if (< _returnvalue _cargo)
        (set `self.Cargo` (- _cargo _returnvalue))
        (else
          ;[1 1 1] if no, send whatever we have
          (bind _output_get_2 (set `self.Amount_to_Transfer` (* _cargo -1.0)))
          (set `self.Cargo` 0.0)))))
  (return _output_get_2))

(fn `UserConstructionScript`)