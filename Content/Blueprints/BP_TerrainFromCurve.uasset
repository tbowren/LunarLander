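; BP_TerrainFromCurve builds a blocky terrain strip from static mesh components, shaped by a float curve.
; The construction script loops up to CubeCount, placing three parallel rows of tall scaled meshes evenly spaced along Y.
; Each height is the floored curve value at that index times a multiplier: HeightScale for the first row, hardcoded for the other two.
; The event graph has no active logic.
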(event `self.ReceiveBeginPlay`)

(event `self.ReceiveActorBeginOverlap`
  (params (OtherActor :type "Actor Object Reference")))

(event `self.ReceiveTick`
  (params (DeltaSeconds :type "Float (single-precision)")))

(fn `UserConstructionScript`
  (for _index (range (+ (`self.CubeCount`) 1))
    (bind _returnvalue (`KismetMathLibrary.Conv_IntToDouble` _index))
    (bind _returnvalue_2 (* _returnvalue 500.0))
    (bind _returnvalue_3 (`KismetMathLibrary.Conv_IntToDouble` (`KismetMathLibrary.FFloor` (`CurveFloat.GetFloatValue` (`self.Curve`) _returnvalue))))
    (`AddComponent|Static Mesh Component_184` :`RelativeTransform` (`KismetMathLibrary.MakeTransform` (`KismetMathLibrary.MakeVector` 0.0 _returnvalue_2 (* _returnvalue_3 (`self.HeightScale`))) (struct) (2.0 2.0 10.0)))
    (`AddComponent|StaticMeshComponent_31930` :`RelativeTransform` (`KismetMathLibrary.MakeTransform` (`KismetMathLibrary.MakeVector` -500.0 _returnvalue_2 (* _returnvalue_3 220.0)) (struct) (2.0 2.0 10.0)))
    (`AddComponent|StaticMeshComponent_46731` :`RelativeTransform` (`KismetMathLibrary.MakeTransform` (`KismetMathLibrary.MakeVector` -1000.0 _returnvalue_2 (* _returnvalue_3 200.0)) (struct) (2.0 2.0 10.0)))))