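; Player ship, a rotate-world movement variant with thrust, fuel and a grab for physics objects below it.
; Both tilt axes share one handler that rotates Ball and builds Momentum, which spins MovementCube each tick, while thrust input drives PhysicsThruster, pivot scale and engine volume.
; Tick drains fuel by throttle, adds the SendPower charge rate and updates both widgets.
; Grab traces down and holds the hit below Ball with a runtime-added PhysicsHandle; cargo functions are stubs.
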(event `self.ReceiveTick`
  (params (DeltaSeconds :type "Float (single-precision)"))
  (bind _movementcube (`self.MovementCube`))
  (bind _maxfuel (`self.MaxFuel`))
  (bind _returnvalue (/ (`self.Fuel`) (`self.MaxFuel`)))
  (bind _returnvalue_2 (`KismetTextLibrary.Conv_DoubleToText` (`KismetMathLibrary.Conv_IntToDouble` (`KismetMathLibrary.Round` (* 100 _returnvalue))) "HalfToEven"))
  ;[1 1 1] TICK
  (`SceneComponent.K2_AddRelativeRotation` _movementcube (`KismetMathLibrary.MakeRot` (.x (`self.Momentum`))) false)
  (`SceneComponent.K2_AddRelativeRotation` _movementcube (`KismetMathLibrary.MakeRot` 0.0 0.0 (.y (`self.Momentum`))) false)
  (bind _returnvalue_3 (- (`self.Fuel`) (* (* DeltaSeconds (stale `InputAxis|MoveThrust` AxisValue)) (`self.Inefficiency`))))
  (if (< _returnvalue_3 0.0)
    (set `self.Fuel` 0.0))
  (bind _returnvalue_4 (+ (`self.ChargeRate`) _returnvalue_3))
  (if (< _returnvalue_4 _maxfuel)
    (set `self.Fuel` _returnvalue_4)
    (else
      (set `self.Fuel` _maxfuel)))
  (bind _aswidget_fuel (cast `/Game/Blueprints/Widget_Fuel` (`WidgetComponent.GetUserWidgetObject` (`self.Widget`))))
  (bind _aswidget_hud (cast `/Game/Blueprints/Widget_HUD` (`WidgetComponent.GetUserWidgetObject` (`self.Widget_HUD`))))
  (`TextBlock.SetText` (`/Game/Blueprints/Widget_Fuel.TextBlock` _aswidget_fuel) _returnvalue_2)
  (`ProgressBar.SetPercent` (`/Game/Blueprints/Widget_Fuel.PB_Fuel` _aswidget_fuel) _returnvalue)
  (`TextBlock.SetText` (`/Game/Blueprints/Widget_HUD.TXT_FuelPercent` _aswidget_hud) _returnvalue_2)
  (if (`self.isGrabbed`)
    (`PhysicsHandleComponent.SetTargetLocationAndRotation` :`self` (`self.PhysicsHandle`) :`NewLocation` (+ (`SceneComponent.K2_GetComponentLocation` (`self.Ball`)) (0.0 0.0 -500.0)))))

(event `self.ReceiveBeginPlay`
  ;[1 1 1] BeginPlay set startig fuel
  (set `self.MaxFuel` (`self.Fuel`)))

(event `InputAction|GrabObject`
  (bind _returnvalue (`SceneComponent.K2_GetComponentLocation` (`self.Ball`)))
  ;[1 1 1] GRAB
  (:`Pressed`
    (set `self.isGrabbed` true)
    (bind _outhit (`KismetSystemLibrary.LineTraceSingleForObjects` :`Start` _returnvalue :`End` (+ _returnvalue (0.0 0.0 -1000.0)) :`ObjectTypes` (`self.PhysicsObjectTypes`) :`DrawDebugType` "ForDuration"))
    (bind _returnvalue_2 (`AddComponent|Physics Handle Component_1`))
    (set `self.PhysicsHandle` _returnvalue_2)
    (bind (_bblockinghit _binitialoverlap _time _location _impactpoint _normal _impactnormal _physmat _hitactor _hitcomponent) (`GameplayStatics.BreakHitResult` _outhit))
    (set `self.PhysicsObject` _hitcomponent)
    (`PhysicsHandleComponent.GrabComponent` (`self.PhysicsHandle`) _hitcomponent "None" _location true))
  (:`Released`
    (set `self.isGrabbed` false)
    (`PhysicsHandleComponent.ReleaseComponent` (`self.PhysicsHandle`))))

(event `InputAxis|MoveThrust`
  (params (AxisValue :type "Float (single-precision)"))
  ;[1 1 1] Thrust
  (set `PhysicsThrusterComponent.ThrustStrength` (* (`self.ThrustForce`) AxisValue -1.0) (`self.PhysicsThruster`))
  (`SceneComponent.SetRelativeScale3D` (`self.ThrustPivot`) (`KismetMathLibrary.MakeVector` 1.0 1.0 (* AxisValue 3.0)))
  ;[1 1 1] Audio
  (`AudioComponent.SetVolumeMultiplier` (`self.Engine_Thrust`) AxisValue))

(event `InputAxis|MoveTiltAway`
  (params (AxisValue :type "Float (single-precision)"))
  (bind _returnvalue (* AxisValue -50.0))
  ;[1 1 1] Roll left/right
  (bind _returnvalue_2 (* (stale `InputAxis|MoveTiltRight` AxisValue) 50.0))
  (`SceneComponent.K2_SetWorldRotation` (`self.Ball`) (`KismetMathLibrary.MakeRot` _returnvalue 0.0 _returnvalue_2) false :!label _label)
  (set `self.Momentum` (+ (`self.Momentum`) (* (* (`KismetMathLibrary.MakeVector` (* _returnvalue 0.01) (* _returnvalue_2 0.01)) (`GameplayStatics.GetWorldDeltaSeconds`)) 0.2))))

(event `InputAxis|MoveTiltRight`
  (params (AxisValue :type "Float (single-precision)"))
  ;[1 1 1] Roll left/right
  (goto _label))

(fn `SendCargo`
  (params (NewParam :type "Float (double-precision)"))
  (returns (CargoOut :type "Float (double-precision)"))
  (return 0.0))

(fn `SendPower`
  (params (NewParam :type "Float (double-precision)"))
  (returns (PowerOut :type "Float (double-precision)"))
  (set `self.ChargeRate` NewParam)
  (return 0.0))

(fn `TransferCargo`
  (params (NewParam :type "Float (double-precision)"))
  (returns (NewParam1 :type "Float (double-precision)"))
  (return 0.0))

(fn `UserConstructionScript`)