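; Cargo depot actor that pulls cargo from an overlapping ship and consumes its stock over time.
; Begin and end overlap toggle a transfer flag that Tick reads to request rate-scaled cargo from the other actor through TransferCargoMessage.
; Transfer stops when the ship runs short or the depot fills; otherwise storage drains, clamped at zero.
; Tick also drives the Widget_Fuel cargo bar; SendCargo, SendPower and TransferCargo are zero-returning stubs.
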(event `self.ReceiveBeginPlay`)

(event `OnComponentBeginOverlap_Event_0`
  (params (OtherActor :type "Actor Object Reference") (OtherComp :type "PrimitiveComponent Object Reference") (OtherBodyIndex :type Integer) (bFromSweep :type Boolean) (SweepResult :type "HitResult Structure (by ref)")))

(event `self.ReceiveActorBeginOverlap`
  (params (OtherActor :type "Actor Object Reference"))
  ;[1 1 1] overlap events
  (set `self.isSendingPower` true))

(event `self.ReceiveActorEndOverlap`
  (params (OtherActor :type "Actor Object Reference"))
  ;[1 1 1] overlap events
  (set `self.isSendingPower` false))

(event `self.ReceiveTick`
  (params (DeltaSeconds :type "Float (single-precision)"))
  (bind _maxcargostorage (`self.MaxCargoStorage`))
  (bind _returnvalue (* (`self.TransferEnergyRate`) DeltaSeconds))
  (bind _aswidget_fuel (cast `/Game/Blueprints/Widget_Fuel` (`WidgetComponent.GetUserWidgetObject` (`self.Widget`))))
  ;[1 1 1] updates Fuel Widget
  (`ProgressBar.SetPercent` (`/Game/Blueprints/Widget_Fuel.PB_Cargo` _aswidget_fuel) (/ (`self.CargoStorage`) (`self.MaxCargoStorage`)))
  ;[1 1 1] If receiving cargo make sure some is being transferred then stop
  (if (`self.isSendingPower`)
    (`|ExecutionSequence`
      (:`then_0`
        (bind _newparam1 (message `/Game/Blueprints/BPI_Emission.TransferCargo` (stale `self.ReceiveActorBeginOverlap` OtherActor) _returnvalue))
        (bind _returnvalue_2 (`KismetMathLibrary.Abs` _newparam1))
        (set `self.CargoStorage` (+ _returnvalue_2 (`self.CargoStorage`)))
        ;[1 1 1] no more cargo available to get
        (if (< _returnvalue_2 _returnvalue)
          (set `self.isSendingPower` false)
          (`KismetSystemLibrary.PrintString` "Ship Empty")
          (else
            ;[1 1 1] if cargo strorage is full , stop
            (if (>= (`self.CargoStorage`) _maxcargostorage)
              (set `self.CargoStorage` _maxcargostorage)
              (set `self.isSendingPower` false)
              (`KismetSystemLibrary.PrintString` "Depot Full"))))))
    (else
      ;[1 1 1] if not receiving, depelete cargo in factory
      (set `self.CargoStorage` (`KismetMathLibrary.FClamp` (- (`self.CargoStorage`) (* DeltaSeconds (`self.UseCargoRate`))) 0.0 (`self.MaxCargoStorage`))))))

(fn `SendCargo`
  (params (NewParam :type "Float (double-precision)"))
  (returns (CargoOut :type "Float (double-precision)"))
  (return 0.0))

(fn `SendPower`
  (params (NewParam :type "Float (double-precision)"))
  (returns (PowerOut :type "Float (double-precision)"))
  (return 0.0))

(fn `TransferCargo`
  (params (NewParam :type "Float (double-precision)"))
  (returns (NewParam1 :type "Float (double-precision)"))
  (return 0.0))

(fn `UserConstructionScript`)