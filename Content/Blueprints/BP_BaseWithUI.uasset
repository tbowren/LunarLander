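; Clickable actor, apparently a base class, that opens a scrollable list UI when its static mesh is clicked.
; The first click adds a Widget_Scrollable_UI to the viewport and sets IsUI to block repeats; the logic to hide it is unwired.
; Each ListItems text gets a Widget_ListItem, whose inner JoyButton, rather than the whole widget, is added to JoyList.
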(event `self.StaticMesh.OnClicked`
  (params (TouchedComponent :type "PrimitiveComponent Object Reference"))
  (if (not (`self.isUI`))
    (`self.CreateJoyUI`)
    (`self.AddListItems`)
    (set `self.isUI` true)))

(event `self.ReceiveActorBeginOverlap`
  (params (OtherActor :type "Actor Object Reference")))

(event `self.ReceiveTick`
  (params (DeltaSeconds :type "Float (single-precision)")))

(fn `AddListItems`
  (for _array_element (`self.ListItems`)
    (bind _createdbutton (`self.CreateButtonAndSetText` _array_element))
    (bind _aswidget (cast `Widget` _createdbutton))
    (`PanelWidget.AddChild` (`/Game/Blueprints/Widget_Scrollable_UI.JoyList` (`self.JoyUI`)) _aswidget)))

(fn `CreateButtonAndSetText`
  (params (Text :type Text))
  (returns (CreatedButton :type "Object Object Reference"))
  (bind _returnvalue (`|CreateWidget` "/Game/Blueprints/Widget_ListItem.Widget_ListItem_C" (`GameplayStatics.GetPlayerController` 0)))
  (set `/Game/Blueprints/Widget_ListItem.TextToDisplay` (`KismetTextLibrary.Conv_TextToString` Text) _returnvalue)
  (`EditableTextBox.SetText` (`/Game/Blueprints/Widget_ListItem.JoyText` _returnvalue) Text)
  (return (`/Game/Blueprints/Widget_ListItem.JoyButton` _returnvalue)))

(fn `CreateJoyUI`
  (bind _returnvalue (`|CreateWidget` "/Game/Blueprints/Widget_Scrollable_UI.Widget_Scrollable_UI_C" (`GameplayStatics.GetPlayerController` 0)))
  (set `self.JoyUI` _returnvalue)
  (`UserWidget.AddToViewport` _returnvalue 0))

(fn `UserConstructionScript`)