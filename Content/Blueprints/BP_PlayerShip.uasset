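; Player ship for a lander-style game with fuel-limited physics thrust, tilt steering and crash or landing outcomes.
; Tick burns fuel from throttle, drives thruster, flame and audio, and updates fuel/cargo HUD bars.
; A downward trace gives altitude, which steps camera distance and, near ground, uses speed to crash or award landing score and fuel before click-to-restart.
; Also provides cargo/power transfer functions and physics-handle grabbing, whose target-follow logic is unwired.
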(event `Key|Gamepad_FaceButton_Bottom`
  (bind _ball (`self.Ball`))
  (:`Pressed`
    (if (`self.isClickedToRestart`) :!label _label
      (set `self.isCrashed` false)
      (set `self.isLanded` false)
      (set `self.isClickedToRestart` false)
      (`SceneComponent.K2_SetWorldLocation` _ball (`self.StartLocation`) false)
      (`PrimitiveComponent.SetMaterial` _ball 0 "/Game/Materials/M_Ship.M_Ship"))))

(event `Key|LeftMouseButton`
  (:`Pressed`
    (goto _label)))

(event `self.ReceiveTick`
  (params (DeltaSeconds :type "Float (single-precision)"))
  (bind _springarm (`self.SpringArm`))
  (bind _throttleaxis (`self.ThrottleAxis`))
  (bind _returnvalue (`SceneComponent.GetComponentVelocity` (`self.Ball`)))
  (bind _returnvalue_2 (`SceneComponent.K2_GetComponentLocation` (`self.Ball`)))
  (bind _returnvalue_3 (- (`self.Fuel`) (* (* DeltaSeconds (`self.ThrottleAxis`)) (`self.Inefficiency`))))
  (if (`self.isCrashed`)
    (`PrimitiveComponent.SetMaterial` (`self.Ball`) 0 "/Game/Materials/M_Ship_Red.M_Ship_Red")
    (set `PhysicsThrusterComponent.ThrustStrength` 0.0 (`self.PhysicsThruster`))
    (`SceneComponent.SetRelativeScale3D` (`self.ThrustPivot`) (1.0 1.0 0.0))
    (else
      (set `self.ThrottleAxis` (stale `InputAxis|MoveThrust` AxisValue))
      ;[1 1 1] Make sure we have fuel in tank but dont go negative
      (set `self.Time` (+ (`self.Time`) DeltaSeconds))
      (if (< _returnvalue_3 0.0)
        (set `self.Fuel` 0.0)
        (else
          (set `self.Fuel` _returnvalue_3)
          ;[1 1 1] Scale and show engine Thrust
          (set `PhysicsThrusterComponent.ThrustStrength` (* (`self.ThrustForce`) _throttleaxis -1.0) (`self.PhysicsThruster`))
          (`SceneComponent.SetRelativeScale3D` (`self.ThrustPivot`) (`KismetMathLibrary.MakeVector` 1.0 1.0 (* _throttleaxis 3.0)))
          ;[1 1 1] Audio
          (`AudioComponent.SetVolumeMultiplier` (`self.Engine_Thrust`) _throttleaxis)))
      ;[1 1 1] Update HUD
      (bind _aswidget_fuel (cast `/Game/Blueprints/Widget_Fuel` (`WidgetComponent.GetUserWidgetObject` (`self.Widget`))))
      (if (not (`self.isCrashed`))
        (`ProgressBar.SetPercent` (`/Game/Blueprints/Widget_Fuel.PB_Fuel` _aswidget_fuel) (/ (`self.Fuel`) (`self.MaxFuel`)))
        (`ProgressBar.SetPercent` (`/Game/Blueprints/Widget_Fuel.PB_Cargo` _aswidget_fuel) (/ (`self.Cargo`) (`self.MaxCargo`))))
      (bind _outhit (`KismetSystemLibrary.LineTraceSingle` _returnvalue_2 (- _returnvalue_2 (0.0 0.0 30000.0)) "TraceTypeQuery1"))
      (bind (_bblockinghit _binitialoverlap _time _location _impactpoint _normal _impactnormal _physmat _hitactor _hitcomponent _hitbonename _hititem _tracestart) (`GameplayStatics.BreakHitResult` _outhit))
      (bind _output_get (set `self.Altitude` (`KismetMathLibrary.VSize` (- _tracestart _impactpoint))))
      (if (> _output_get 12000.0)
        (set `SpringArmComponent.TargetArmLength` 24000.0 _springarm)
        (elif (< _output_get 5000.0)
          (set `SpringArmComponent.TargetArmLength` 5000.0 _springarm)
          (if (< _output_get 128.0)
            (if (> (`KismetMathLibrary.VSize` _returnvalue) 750.0)
              (`KismetSystemLibrary.PrintString` "CRASH")
              (set `self.Fuel` 0.0)
              (set `self.isCrashed` true)
              (set `self.CrashedVel` _returnvalue)
              (set `self.ThrottleAxis` 0.0)
              (`KismetSystemLibrary.Delay` 2.0)
              (set `self.isClickedToRestart` true)
              (elif (not (`self.isCrashed`))
                (`/Engine/EditorBlueprintResources/StandardMacros.DoOnce` false :!label _label_2
                  (:`Completed`
                    (set `self.isLanded` true)
                    (set `self.Score` (+ (`self.Score`) 10))
                    (set `self.Fuel` (+ (`self.Fuel`) 50.0))
                    (`KismetSystemLibrary.Delay` 2.0)
                    (set `self.isClickedToRestart` true))))))
          (else
            (set `SpringArmComponent.TargetArmLength` 12000.0 _springarm)))))))

(event `InputAxis|MoveThrust`
  (params (AxisValue :type "Float (single-precision)"))
  ;[1 1 1] Thrust
)

(event `Key|LeftMouseButton`
  (:`Pressed`
    (goto _label_2 :!via `Reset`)))

(event `Key|Gamepad_FaceButton_Bottom`
  (:`Pressed`
    (goto _label_2 :!via `Reset`)))

(event `self.ReceiveBeginPlay`
  ;[1 1 1] Comment
  (set `self.MaxFuel` (`self.Fuel`))
  (set `self.StartLocation` (`self.K2_GetActorLocation`)))

(event `InputAction|GrabObject`
  (bind _returnvalue (`SceneComponent.K2_GetComponentLocation` (`self.Ball`)))
  ;[1 1 1] Grab
  (:`Pressed`
    (set `self.isGrabbed` true)
    (bind _outhit (`KismetSystemLibrary.LineTraceSingleForObjects` _returnvalue (+ _returnvalue (0.0 0.0 -1000.0)) (`self.PhysicsObjectTypes`)))
    (bind _returnvalue_2 (`AddComponent|Physics Handle Component_1`))
    (set `self.PhysicsHandle` _returnvalue_2)
    (bind (_bblockinghit _binitialoverlap _time _location _impactpoint _normal _impactnormal _physmat _hitactor _hitcomponent) (`GameplayStatics.BreakHitResult` _outhit))
    (set `self.PhysicsObject` _hitcomponent)
    (`PhysicsHandleComponent.GrabComponent` (`self.PhysicsHandle`) _hitcomponent "None" _location true))
  (:`Released`
    (set `self.isGrabbed` false)
    (`PhysicsHandleComponent.ReleaseComponent` (`self.PhysicsHandle`))))

(event `InputAxis|MoveTiltAway`
  (params (AxisValue :type "Float (single-precision)"))
  (bind _ball (`self.Ball`))
  ;[1 1 1] Roll / Tilt
  (if (not (`self.isCrashed`)) :!label _label_3
    (`SceneComponent.K2_SetWorldRotation` _ball (`KismetMathLibrary.RInterpTo` (`SceneComponent.K2_GetComponentRotation` _ball) (`KismetMathLibrary.MakeRot` (* AxisValue -50.0) 0.0 (* (stale `InputAxis|MoveTiltRight` AxisValue) (`KismetMathLibrary.FClamp` (* (`KismetMathLibrary.Abs` (.y (`SceneComponent.GetComponentVelocity` (`self.Ball`)))) 0.5) 50.0 90.0))) 1.0 (`self.ShipRotate Drag`)) false)))

(event `InputAxis|MoveTiltRight`
  (params (AxisValue :type "Float (single-precision)"))
  ;[1 1 1] Roll / Tilt
  (goto _label_3))

(event `self.CollisionBox.OnComponentHit`
  (params (OtherActor :type "Actor Object Reference") (OtherComp :type "PrimitiveComponent Object Reference") (NormalImpulse :type "Vector Structure") (Hit :type "HitResult Structure (by ref)"))
  (`/Engine/EditorBlueprintResources/StandardMacros.DoOnce` false))

(fn `SendCargo`
  (params (NewParam :type "Float (double-precision)"))
  (returns (CargoOut :type "Float (double-precision)"))
  ;[1 1 1] Make sure not over filled
  (bind _output_get (set `self.Cargo` (+ NewParam (`self.Cargo`))))
  (if (>= _output_get (`self.MaxCargo`))
    (bind _output_get_2 (set `self.FuelTken` NewParam))
    (else
      (set `self.FuelTken` 0.0)))
  (return _output_get_2))

(fn `SendPower`
  (params (NewParam :type "Float (double-precision)"))
  (returns (PowerOut :type "Float (double-precision)"))
  (bind _maxfuel (`self.MaxFuel`))
  ;[1 1 1] Make sure not over filled
  (bind _output_get (set `self.Fuel` (+ NewParam (`self.Fuel`))))
  (if (>= _output_get _maxfuel)
    (set `self.Fuel` _maxfuel)
    (else
      (bind _output_get_2 (set `self.FuelTken` NewParam))))
  (return _output_get_2))

(fn `TransferCargo`
  (params (NewParam :type "Float (double-precision)"))
  (returns (NewParam1 :type "Float (double-precision)"))
  (bind _cargo (`self.Cargo`))
  (bind _returnvalue (`KismetMathLibrary.Abs` (`self.Amount_to_Transfer`)))
  (bind _output_get (set `self.Amount_to_Transfer` NewParam))
  ;[1 1 1] if value is positive, moving cargo to ship
  (if (not (> _output_get 0.0))
    ;[1 1 1] if negative,  taking cargo OFF ship
    (if (< (`self.Amount_to_Transfer`) 0.0)
      ;[1 1 1] Do we have enough cargo to send?
      (if (< _returnvalue _cargo)
        (set `self.Cargo` (- _cargo _returnvalue))
        (else
          ;[1 1 1] if no, send whatever we have
          (bind _output_get_2 (set `self.Amount_to_Transfer` (* _cargo -1.0)))
          (set `self.Cargo` 0.0)))))
  (return _output_get_2))

(fn `UserConstructionScript`)